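; Paper2D actor of an up-and-down type that moves on an InterpToMovement component and changes its sprite animation to match its travel direction.
; Each time the movement reverses, a FlipFlop alternates the PaperFlipbook between the Front and Back flipbooks, starting with Front on the first reversal.
; The BeginPlay, overlap and Tick events are disabled stubs, and the construction script only calls its parent.
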(event OnInterptoReverse(InterpToMovement)
  (params (ImpactResult :type Hit%20Result%20Structure%20%28by%20ref%29) (Time :type Float%20%28single-precision%29))
  (Utilities|FlowControl|FlipFlop
    (:A
      (Sprite|SetFlipbook (Variables|Default|GetPaperFlipbook) "/Game/character/Enemies/2/front.front"))
    (:B
      (Sprite|SetFlipbook (Variables|Default|GetPaperFlipbook) "/Game/character/Enemies/2/back.back"))))

(event EventBeginPlay
  (|CallParentFunction) ; This node is disabled and will not be called.\nDrag off pins to build functionality.
)

(event Collision|EventActorBeginOverlap
  (params (OtherActor :type Actor%20Object%20Reference))
  (|CallParentFunction OtherActor) ; This node is disabled and will not be called.\nDrag off pins to build functionality.
)

(event EventTick
  (params (DeltaSeconds :type Float%20%28single-precision%29))
  (|CallParentFunction DeltaSeconds) ; This node is disabled and will not be called.\nDrag off pins to build functionality.
)

(fn ConstructionScript
  (|CallParentFunction))