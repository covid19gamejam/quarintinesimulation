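; Child enemy Blueprint of a side-to-side type, with a Paper2D flipbook sprite and InterpToMovement.
; Each time the movement reverses, a FlipFlop alternates the flipbook's world rotation between zero and a 180-degree turn, flipping the sprite.
; The BeginPlay, overlap and Tick events are disabled stubs, and the construction script only calls the parent.
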(event OnInterptoReverse(InterpToMovement)
  (params (ImpactResult :type Hit%20Result%20Structure%20%28by%20ref%29) (Time :type Float%20%28single-precision%29))
  (bind _paperflipbook (Variables|Default|GetPaperFlipbook))
  (Utilities|FlowControl|FlipFlop
    (:A
      (Transformation|SetWorldRotation _paperflipbook "0, 0, 0" false false))
    (:B
      (Transformation|SetWorldRotation _paperflipbook "0,180.000000, 0" false false))))

(event EventBeginPlay
  (|CallParentFunction) ; This node is disabled and will not be called.\nDrag off pins to build functionality.
)

(event Collision|EventActorBeginOverlap
  (params (OtherActor :type Actor%20Object%20Reference))
  (|CallParentFunction OtherActor) ; This node is disabled and will not be called.\nDrag off pins to build functionality.
)

(event EventTick
  (params (DeltaSeconds :type Float%20%28single-precision%29))
  (|CallParentFunction DeltaSeconds) ; This node is disabled and will not be called.\nDrag off pins to build functionality.
)

(fn ConstructionScript
  (|CallParentFunction))